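; BP_OldConductor is an actor that uses Quartz to play a drum track in time with a musical clock.
; On BeginPlay it creates a 4/4 clock at a fixed tempo, subscribes to beat events and queues the track on a bar boundary.
; The clock starts once, when the quantized play command reports Queued, so playback and clock begin together.
; BarEvent prints the beat number for debugging.
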(event Custom|BarEvent
  (params (ClockName :type Name) (QuantizationType :type EQuartzCommandQuantization%20Enum :default "Bar") (NumBars :type Integer) (Beat :type Integer) (BeatFraction :type Float%20%28single-precision%29))
  (Development|PrintString (Utilities|String|BuildString(Integer) "Beat: " "" Beat) true true "(R=0.000000,G=0.660000,B=1.000000,A=1.000000)" 2.0 "Beat"))

(event Custom|Event%20QueueMusic
  (bind _returnvalue (Audio|CreateSound2D "/Game/Tonic/Static/Audio/A_Drum_Track_105.A_Drum_Track_105" 1.0 1.0 0.0 0))
  (Audio|Components|Audio|PlayQuantized _returnvalue (Variables|Default|GetClockHandle) (Utilities|Struct|MakeQuartzQuantizationBoundary "Bar" 1.0 "CurrentTimeRelative") (delegate Custom|Event%20QuantizedMusic)))

(event Custom|Event%20QuantizedMusic
  (params (EventType :type EQuartzCommandDelegateSubType%20Enum :default "CommandOnFailedToQueue") (Name :type Name))
  (switch Utilities|FlowControl|Switch|SwitchonEQuartzCommandDelegateSubType EventType
    (:CommandOnQueued
      (Utilities|FlowControl|DoOnce false
        (:Completed
          (Class|QuartzClockHandle|StartClock (Variables|Default|GetClockHandle)))))))

(event EventBeginPlay
  (bind _returnvalue (Class|QuartzSubsystem|CreateNewClock (WorldSubsystems|GetQuartzSubsystem) "TestClock" (Utilities|Struct|MakeQuartzClockSettings (Utilities|Struct|MakeQuartzTimeSignature 4 "QuarterNote") false) false))
  (bind _output_get (Variables|Default|SetClockHandle _returnvalue))
  (bind _clockhandle (Class|QuartzClockHandle|SetBeatsPerMinute :self _output_get :BeatsPerMinute 105.0))
  (Class|QuartzClockHandle|SubscribetoQuantizationEvent _clockhandle "Beat" (EventDispatchers|CreateEvent :!event Custom|BarEvent))
  (CallFunction|EventQueueMusic))

(event Collision|EventActorBeginOverlap
  (params (OtherActor :type Actor%20Object%20Reference)))

(event EventTick
  (params (DeltaSeconds :type Float%20%28single-precision%29)))

(fn ConstructionScript)