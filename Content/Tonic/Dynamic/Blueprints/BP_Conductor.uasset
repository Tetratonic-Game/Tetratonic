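; Conductor Blueprint that starts a music track on a Quartz clock and reports beats.
; When Quartz is ready, it creates a 2D sound from Track and queues playback quantized to a bar, relative to the current time.
; OnBeat only prints the beat number for debugging.
; The quantization callback handles only the Queued event, which reaches a DoOnce with nothing after it.
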(event Custom|Event%20QuantizedMusic
  (params (EventType :type EQuartzCommandDelegateSubType%20Enum :default "CommandOnFailedToQueue") (Name :type Name))
  (switch Utilities|FlowControl|Switch|SwitchonEQuartzCommandDelegateSubType EventType
    (:CommandOnQueued
      (Utilities|FlowControl|DoOnce false))))

(event EventBeginPlay)

(event Collision|EventActorBeginOverlap
  (params (OtherActor :type Actor%20Object%20Reference)))

(event EventTick
  (params (DeltaSeconds :type Float%20%28single-precision%29)))

(event EventOnBeat
  (params (ClockName :type Name :default "None") (QuantizationType :type EQuartzCommandQuantization%20Enum :default "Bar") (NumBars :type Integer) (Beat :type Integer) (BeatFraction :type Float%20%28single-precision%29))
  (Development|PrintString (Utilities|String|BuildString(Integer) "Beat: " "" Beat) true true "(R=0.000000,G=0.660000,B=1.000000,A=1.000000)" 2.0 "Beat"))

(event EventOnQuartzReady
  (bind _returnvalue (Audio|CreateSound2D (Variables|Conductor|GetTrack) 1.0 1.0 0.0 0))
  (Audio|Components|Audio|PlayQuantized _returnvalue (Variables|Default|GetQuartzClock) (Utilities|Struct|MakeQuartzQuantizationBoundary "Bar" 1.0 "CurrentTimeRelative") (delegate Custom|Event%20QuantizedMusic)))

(fn ConstructionScript)