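; BP_Player is a player Blueprint whose Sphere component shifts upward while the IA_Up input action is held.
; Pressing the action places the Sphere at Origin plus an up vector scaled by InputDisplacement, read from the GM_Track game mode.
; Releasing it, like BeginPlay, snaps the Sphere back to Origin.
; Both moves set relative location instantly without sweep, so only the component moves.
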(event Input|EnhancedActionEvents|EnhancedInputActionIA_Up
  (params (ActionValue :type Boolean) (ElapsedSeconds :type Float%20%28double-precision%29) (TriggeredSeconds :type Float%20%28double-precision%29) (InputAction :type Input%20Action%20Object%20Reference :default "/Game/Dynamic/IA_Up.IA_Up"))
  (:Started
    (CallFunction|DisplaceSphere "0.000000,0.000000,1.000000"))
  (:Completed
    (CallFunction|ReturntoOrigin)))

(event EventBeginPlay
  (CallFunction|ReturntoOrigin))

(fn ConstructionScript)

(fn ReturntoOrigin
  (Transformation|SetRelativeLocation (Variables|Default|GetSphere) (Variables|Default|GetOrigin) false false))

(fn DisplaceSphere
  (params (DirectionNormal :type Vector))
  (bind _asgm_track (Utilities|Casting|CastToGM_Track (Game|GetGameMode)))
  (Transformation|SetRelativeLocation (Variables|Default|GetSphere) (+ (* DirectionNormal (Variables|/Game/Dynamic/GM_Track.GM_Track_C|GetInputDisplacement _asgm_track)) (Variables|Default|GetOrigin)) false false))