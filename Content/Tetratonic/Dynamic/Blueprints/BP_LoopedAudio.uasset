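; BP_LoopedAudio is an actor that plays an assigned wave asset as looped 2D audio with fade-in and fade-out.
; BeginPlay creates a sound from the MSS_LoopedSound MetaSound, passes in the wave, starts playback and drives its Gain parameter with a start timeline.
; StopAudio drives Gain with a second timeline, then stops and destroys the audio component and the actor itself.
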(event Custom|Stop%20Audio
  (bind _metasound (Variables|Default|GetMetasound))
  (if (Utilities|IsValid _metasound)
    (bind _gainvalue (Timeline|StopAudioTimeline PlayFromStart)
      (:Update
        (Audio|Parameter|SetFloatParameter _metasound "Gain" _gainvalue :!class /Script/Engine.AudioComponent))
      (:Finished
        (Audio|Components|Audio|Stop _metasound)
        (Components|DestroyComponent _metasound)
        (Actor|DestroyActor)))))

(event EventBeginPlay
  (bind _returnvalue (Audio|CreateSound2D "/Game/Tetratonic/Dynamic/Metasounds/MSS_LoopedSound.MSS_LoopedSound" 1.0 1.0 0.0 0))
  (bind _output_get (Variables|Default|SetMetasound _returnvalue))
  (Class|AudioComponent|SetWaveParameter _output_get "Wave Asset" (Variables|Default|GetWave%20Asset))
  (Audio|Components|Audio|Play _returnvalue 0.0)
  (bind _gainvalue (Timeline|StartAudioTimeline PlayFromStart)
    (:Update
      (Audio|Parameter|SetFloatParameter _returnvalue "Gain" _gainvalue :!class /Script/Engine.AudioComponent))))

(fn ConstructionScript)