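; BP_Instrument is an actor that plays looped chord notes in time with the track game mode's Quartz clock.
; TriggerNote maps a chord position and the current bar in a four-bar cycle through ChordNoteMap to a sound, rounding up late in beat four.
; Each beat re-triggers the active position to follow chord changes.
; It spawns a new BP_LoopedAudio only when the sound changes, stopping the previous one.
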(event Custom|StartSound
  (params (WaveAsset :type Sound%20Wave%20Object%20Reference))
  (CallFunction|StopSound)
  (bind _returnvalue (Game|SpawnActorfromClass "/Game/Tetratonic/Dynamic/Blueprints/BP_LoopedAudio.BP_LoopedAudio_C" (Transformation|GetActorTransform) "AlwaysSpawn" "MultiplyWithRoot" 0 WaveAsset 0))
  (Variables|Default|SetCurrentSound _returnvalue))

(event Custom|StopSound
  (bind _currentsound (Variables|Default|GetCurrentSound))
  (if (Utilities|IsValid _currentsound)
    (Default|StopAudio _currentsound)))

(event Custom|OnBeat
  (params (ClockName :type Name) (QuantizationType :type EQuartzCommandQuantization%20Enum :default "Bar") (NumBars :type Integer) (Beat :type Integer) (BeatFraction :type Float%20%28single-precision%29))
  (CallFunction|TriggerNextChord))

(event EventBeginPlay
  (bind _astrack_game_mode (Utilities|Casting|CastToTrackGameMode (Game|GetGameMode)))
  (bind _output_get (Variables|Default|SetTrackGameMode _astrack_game_mode))
  (Class|QuartzClockHandle|SubscribetoQuantizationEvent (Variables|/Script/Tetratonic.TrackGameMode|GetQuartzClock _output_get) "Beat" (delegate Custom|OnBeat)))

(fn ConstructionScript)

(fn TriggerNote
  (params (ChordPosition :type EChordPosition%20Enum :default "NewEnumerator0"))
  (bind _output_get (Variables|Default|SetCurrentChordPosition ChordPosition))
  (bind _noteindex (CallFunction|GetNoteIndexfromChordPosition _output_get))
  (CallFunction|SetActiveNote _noteindex))

(fn GetNoteIndexfromChordPosition
  (params (Chord%20Position :type EChordPosition%20Enum :default "NewEnumerator0"))
  (bind _trackgamemode (Variables|Default|GetTrackGameMode))
  (bind (_bars _beat _beatfraction) (Class|TrackGameMode|GetCorrectedTimestamp _trackgamemode))
  (return (+ (* (Math|Integer|%(Integer) (- _bars (Math|Conversions|ToInteger(Boolean) (not (and (== _beat 4) (> _beatfraction 0.8))))) 4) 4) (Math|Conversions|ToInteger(Byte) Chord%20Position))))

(fn StopActiveSound
  (CallFunction|StopSound)
  (Variables|Default|SetCurrentNoteIndex -1)
  (Variables|Default|SetCurrentSoundIndex -1))

(fn SetActiveNote
  (params (NoteIndex :type Integer))
  (bind _chordnotemap (Variables|Default|GetChordNoteMap))
  (bind _output (Utilities|Array|Get(acopy) _chordnotemap NoteIndex))
  (if (== (Variables|Default|GetCurrentSoundIndex) _output)
    (Variables|Default|SetCurrentNoteIndex NoteIndex)
    (else
      (Variables|Default|SetCurrentNoteIndex NoteIndex)
      (Variables|Default|SetCurrentSoundIndex _output)
      (CallFunction|StartSound (Utilities|Array|Get(acopy) (Variables|Default|GetSounds) _output)))))

(fn TriggerNextChord
  (if (not (== (Variables|Default|GetCurrentNoteIndex) -1))
    (CallFunction|TriggerNote (Variables|Default|GetCurrentChordPosition))))