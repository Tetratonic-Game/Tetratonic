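; BP_LineAdversary is a line-shaped adversary actor with start and end neutral caps whose opacity can be animated.
; The construction script gives each cap its own dynamic instance of M_GameplayNeutral.
; StartNeutral and EndNeutral events each play a timeline from the start that drives that cap material's Opacity parameter, so the two ends animate independently.
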(event Custom|Event%20Start%20Neutral
  (bind _opacity (Timeline|StartCapTimeline PlayFromStart)
    (:Update
      (Rendering|Material|SetScalarParameterValue (Variables|Default|GetStartNeutralMaterial) "Opacity" _opacity :!class /Script/Engine.MaterialInstanceDynamic))))

(event Custom|Event%20End%20Neutral
  (bind _opacity (Timeline|EndCapTimeline PlayFromStart)
    (:Update
      (Rendering|Material|SetScalarParameterValue (Variables|Default|GetEndNeutralMaterial) "Opacity" _opacity :!class /Script/Engine.MaterialInstanceDynamic))))

(event EventBeginPlay)

(event Collision|EventActorBeginOverlap
  (params (OtherActor :type Actor%20Object%20Reference)))

(event EventTick
  (params (DeltaSeconds :type Float%20%28single-precision%29)))

(fn ConstructionScript
  (bind _startneutralcap (Variables|Default|GetStartNeutralCap))
  (bind _endneutralcap (Variables|Default|GetEndNeutralCap))
  (bind _returnvalue (Rendering|Material|CreateDynamicMaterialInstance _startneutralcap 0 "/Game/Tetratonic/Static/Materials/M_GameplayNeutral.M_GameplayNeutral" "None" :!class /Script/Engine.PrimitiveComponent))
  (bind _output_get (Variables|Default|SetStartNeutralMaterial _returnvalue))
  (Rendering|Material|SetMaterial _startneutralcap 0 _output_get)
  (bind _returnvalue_2 (Rendering|Material|CreateDynamicMaterialInstance _endneutralcap 0 "/Game/Tetratonic/Static/Materials/M_GameplayNeutral.M_GameplayNeutral" "None" :!class /Script/Engine.PrimitiveComponent))
  (bind _output_get_2 (Variables|Default|SetEndNeutralMaterial _returnvalue_2))
  (Rendering|Material|SetMaterial _endneutralcap 0 _output_get_2))