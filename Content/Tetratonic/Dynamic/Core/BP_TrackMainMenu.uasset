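; Main menu track Blueprint for Tetratonic that shows the menu widget and pulses it in time with the music clock.
; On BeginPlay it creates WBP_MainMenu, shows the mouse cursor and subscribes to Quartz clock beat quantization events.
; Each beat calls OnPulse on the widget.
; ReturntoMainMenu repeats the same setup with a new widget instance and its own beat callback.
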(event Custom|OnReturnBeat
  (params (ClockName :type Name) (QuantizationType :type EQuartzCommandQuantization%20Enum :default "Bar") (NumBars :type Integer) (Beat :type Integer) (BeatFraction :type Float%20%28single-precision%29))
  (Default|OnPulse (stale Custom|Return%20to%20Main%20Menu _returnvalue)))

(event Custom|Return%20to%20Main%20Menu
  (bind _returnvalue (UserInterface|CreateWidget "/Game/Tetratonic/Dynamic/UI/HUDs/WBP_MainMenu.WBP_MainMenu_C" (Game|GetPlayerController 0)))
  (UserInterface|Viewport|AddtoViewport _returnvalue 0)
  (Variables|/Script/Engine.PlayerController|SetbShowMouseCursor (Game|GetPlayerController 0) true)
  (Class|QuartzClockHandle|SubscribetoQuantizationEvent (Variables|Default|GetQuartzClock) "Beat" (delegate Custom|OnReturnBeat)))

(event Custom|OnBeat
  (params (ClockName :type Name) (QuantizationType :type EQuartzCommandQuantization%20Enum :default "Bar") (NumBars :type Integer) (Beat :type Integer) (BeatFraction :type Float%20%28single-precision%29))
  (Default|OnPulse (stale EventBeginPlay _returnvalue)))

(event EventBeginPlay
  (bind _returnvalue (UserInterface|CreateWidget "/Game/Tetratonic/Dynamic/UI/HUDs/WBP_MainMenu.WBP_MainMenu_C" (Game|GetPlayerController 0)))
  (UserInterface|Viewport|AddtoViewport _returnvalue 0)
  (Variables|/Script/Engine.PlayerController|SetbShowMouseCursor (Game|GetPlayerController 0) true)
  (Class|QuartzClockHandle|SubscribetoQuantizationEvent (Variables|Default|GetQuartzClock) "Beat" (delegate Custom|OnBeat)))

(fn ConstructionScript)