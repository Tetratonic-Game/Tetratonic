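; Player pawn for a rhythm game that jumps to four directional playfield positions and triggers notes on the BP_Instrument.
; An input queue gives the latest held direction priority, returning to origin and stopping the sound when all are released.
; Construction offsets the playfields by the TrackGameMode radius.
; Collider hits show accuracy fly text at the nearest widget and report combo increases, while a timeline pulses the mesh on beat.
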(event Input|EnhancedActionEvents|EnhancedInputActionIA_Up
  (params (ActionValue :type Boolean) (ElapsedSeconds :type Float%20%28double-precision%29) (TriggeredSeconds :type Float%20%28double-precision%29) (InputAction :type Input%20Action%20Object%20Reference :default "/Game/Tetratonic/Dynamic/Input/IA_Up.IA_Up"))
  (:Started
    (CallFunction|HandleStartedDirectionalInput InputAction))
  (:Ongoing
    (bind _bshoulddisplace (CallFunction|HandleOngoingDirectionalInput InputAction (Math|Vector|VectorUp)))
    (if _bshoulddisplace
      (bind _returnvalue (Class|PlayerPawn|SetCurrentPosition "Top"))
      (if _returnvalue
        (Default|TriggerNote (Variables|Default|GetInstrument) "NewEnumerator3"))))
  (:Completed
    (CallFunction|HandleCompletedDirectionalInput InputAction)))

(event Input|EnhancedActionEvents|EnhancedInputActionIA_Left
  (params (ActionValue :type Boolean) (ElapsedSeconds :type Float%20%28double-precision%29) (TriggeredSeconds :type Float%20%28double-precision%29) (InputAction :type Input%20Action%20Object%20Reference :default "/Game/Tetratonic/Dynamic/Input/IA_Left.IA_Left"))
  (:Started
    (CallFunction|HandleStartedDirectionalInput InputAction))
  (:Ongoing
    (bind _bshoulddisplace (CallFunction|HandleOngoingDirectionalInput InputAction (Class|KismetMathLibrary|VectorLeft)))
    (if _bshoulddisplace
      (bind _returnvalue (Class|PlayerPawn|SetCurrentPosition "Left"))
      (if _returnvalue
        (Default|TriggerNote (Variables|Default|GetInstrument) "NewEnumerator1"))))
  (:Completed
    (CallFunction|HandleCompletedDirectionalInput InputAction)))

(event Input|EnhancedActionEvents|EnhancedInputActionIA_Down
  (params (ActionValue :type Boolean) (ElapsedSeconds :type Float%20%28double-precision%29) (TriggeredSeconds :type Float%20%28double-precision%29) (InputAction :type Input%20Action%20Object%20Reference :default "/Game/Tetratonic/Dynamic/Input/IA_Down.IA_Down"))
  (:Started
    (CallFunction|HandleStartedDirectionalInput InputAction))
  (:Ongoing
    (bind _bshoulddisplace (CallFunction|HandleOngoingDirectionalInput InputAction (Math|Vector|VectorDown)))
    (if _bshoulddisplace
      (bind _returnvalue (Class|PlayerPawn|SetCurrentPosition "Bottom"))
      (if _returnvalue
        (Default|TriggerNote (Variables|Default|GetInstrument) "NewEnumerator0"))))
  (:Completed
    (CallFunction|HandleCompletedDirectionalInput InputAction)))

(event Input|EnhancedActionEvents|EnhancedInputActionIA_Right
  (params (ActionValue :type Boolean) (ElapsedSeconds :type Float%20%28double-precision%29) (TriggeredSeconds :type Float%20%28double-precision%29) (InputAction :type Input%20Action%20Object%20Reference :default "/Game/Tetratonic/Dynamic/Input/IA_Right.IA_Right"))
  (:Started
    (CallFunction|HandleStartedDirectionalInput InputAction))
  (:Ongoing
    (bind _bshoulddisplace (CallFunction|HandleOngoingDirectionalInput InputAction (Class|KismetMathLibrary|VectorRight)))
    (if _bshoulddisplace
      (bind _returnvalue (Class|PlayerPawn|SetCurrentPosition "Right"))
      (if _returnvalue
        (Default|TriggerNote (Variables|Default|GetInstrument) "NewEnumerator2"))))
  (:Completed
    (CallFunction|HandleCompletedDirectionalInput InputAction)))

(event EventHandleCollider
  (params (Accuracy :type EAccuracyType%20Enum :default "Okay") (bDidIncreaseCombo :type Boolean) (OverlapLocation :type Vector :default "0, 0, 0"))
  (bind _flytextwidget (CallFunction|GetClosestFlyTextWidget OverlapLocation))
  (if bDidIncreaseCombo
    (Default|OnComboIncrease (Variables|Default|GetGameplayWidget)))
  (Variables|/Game/Tetratonic/Dynamic/UI/Widgets/WBP_FlyText.WBP_FlyText_C|SetFlyTextContent _flytextwidget (Utilities|Text|ToText(String) (Utilities|String|EnumtoString Accuracy)))
  (Default|PlayFlyText _flytextwidget))

(event EventOnBeat
  (params (ClockName :type Name :default "None") (QuantizationType :type EQuartzCommandQuantization%20Enum :default "Bar") (NumBars :type Integer) (Beat :type Integer) (BeatFraction :type Float%20%28single-precision%29))
  (bind _scaletrack (Timeline|Timeline PlayFromStart)
    (:Update
      (Transformation|SetRelativeScale3D (Variables|Default|GetPlayerMesh) _scaletrack))))

(event EventBeginPlay
  (bind _bottomflytext (Variables|Default|GetBottomFlyText))
  (bind _rightflytext (Variables|Default|GetRightFlyText))
  (bind _centerflytext (Variables|Default|GetCenterFlyText))
  (bind _topflytext (Variables|Default|GetTopFlyText))
  (bind _leftflytext (Variables|Default|GetLeftFlyText))
  (Class|PlayerPawn|ReturntoOrigin)
  (bind _returnvalue (Actor|GetActorOfClass "/Game/Tetratonic/Dynamic/Blueprints/BP_Instrument.BP_Instrument_C"))
  (if (Utilities|IsValid _returnvalue)
    (Variables|Default|SetInstrument _returnvalue)
    (Variables|Default|SetFlyTextLocationMap (Utilities|Map|MakeMap _centerflytext (Transformation|GetWorldLocation _centerflytext) _topflytext (Transformation|GetWorldLocation _topflytext) _leftflytext (Transformation|GetWorldLocation _leftflytext) _bottomflytext (Transformation|GetWorldLocation _bottomflytext) _rightflytext (Transformation|GetWorldLocation _rightflytext)))))

(fn ConstructionScript
  (bind _astrack_game_mode (Utilities|Casting|CastToTrackGameMode (Game|GetGameMode))
    (:then
      (Variables|Default|SetInputDisplacement (Class|TrackGameMode|GetPlayfieldRadius _astrack_game_mode)))
    (:CastFailed
      (Utilities|String|LogString "Player Pawn construction script does not have TrackGameMode, using default Input Displacement.")))
  (CallFunction|SetPlayfieldComponentOffset (Variables|Default|GetTopPlayfield) (Math|Vector|VectorUp))
  (CallFunction|SetPlayfieldComponentOffset (Variables|Default|GetLeftPlayfield) (Class|KismetMathLibrary|VectorLeft))
  (CallFunction|SetPlayfieldComponentOffset (Variables|Default|GetRightPlayfield) (Class|KismetMathLibrary|VectorRight))
  (CallFunction|SetPlayfieldComponentOffset (Variables|Default|GetBottomPlayfield) (Math|Vector|VectorDown)))

(fn SetPlayfieldComponentOffset
  (params (Component :type Scene%20Component%20Object%20Reference) (Direction :type Vector))
  (Transformation|SetRelativeLocation Component (* Direction (Variables|Default|GetInputDisplacement)) false false))

(fn HandleOngoingDirectionalInput
  (params (InputAction :type Object%20Object%20Reference) (Direction :type Vector))
  (bind _inputqueue (Variables|Default|GetInputQueue))
  (bind _returnvalue (Utilities|Array|LastIndex _inputqueue))
  (bind _output (Utilities|Array|Get(acopy) _inputqueue _returnvalue))
  (bind _returnvalue_2 (== _output InputAction))
  (if _returnvalue_2
    (Class|PlayerPawn|DisplacePawn Direction))
  (return _returnvalue_2))

(fn HandleCompletedDirectionalInput
  (params (InputAction :type Input%20Action%20Object%20Reference%20%28by%20ref%29))
  (Utilities|Array|RemoveItem (Variables|Default|GetInputQueue) InputAction)
  (if (== 0 (Utilities|Array|Length (Variables|Default|GetInputQueue)))
    (Class|PlayerPawn|ReturntoOrigin)
    (Default|StopActiveSound (Variables|Default|GetInstrument))))

(fn HandleStartedDirectionalInput
  (params (InputAction :type Input%20Action%20Object%20Reference%20%28by%20ref%29))
  (Utilities|Array|Add (Variables|Default|GetInputQueue) InputAction))

(fn GetClosestFlyTextWidget
  (params (Overlap%20Location :type Vector))
  (bind _flytextlocationmap (Variables|Default|GetFlyTextLocationMap))
  (bind _keys (Utilities|Map|Keys _flytextlocationmap))
  (bind _values (Utilities|Map|Values _flytextlocationmap))
  (for (_array_element _array_index) _values
    (if (< (Math|Vector|Distance(Vector) _array_element Overlap%20Location) (LocalVariables|GetClosestDistance))
      (LocalVariables|SetClosestDistance (Math|Vector|Distance(Vector) _array_element Overlap%20Location))
      (LocalVariables|SetClosestWidgetIndex _array_index)))
  (bind _aswbp_fly_text (Utilities|Casting|CastToWBP_FlyText (UserInterface|GetUserWidgetObject (Utilities|Array|Get(acopy) _keys (LocalVariables|GetClosestWidgetIndex)))))
  (return _aswbp_fly_text))